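; BP_animal is an animal Blueprint that holds a next target location for an AI-controlled animal.
; On BeginPlay it casts its controller to AIC_animal and stores it as AnimalController.
; The FindNextTargetLocation event caches the result of FindTargetLocation, and GetNextTargetLocation returns that cached value.
; FindTargetLocation is a stub that returns the zero vector, and this file contains no movement logic.
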(event EventFindNextTargetLocation
  (bind _targetlocation (CallFunction|FindTargetLocation))
  (Variables|Default|SetnextTargetLocation _targetlocation))

(event EventBeginPlay
  (bind _asaic_animal (Utilities|Casting|CastToAIC_animal (AI|GetAIController self)))
  (Variables|Default|SetanimalController _asaic_animal))

(fn ConstructionScript)

(fn FindTargetLocation
  (return "0, 0, 0"))

(fn GetNextTargetLocation
  (return (Variables|Default|GetnextTargetLocation)))