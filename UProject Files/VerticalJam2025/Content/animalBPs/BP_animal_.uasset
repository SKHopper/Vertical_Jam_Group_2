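; Animal Blueprint that acts as an AI-controlled creature, caching its AIC_animal controller on BeginPlay.
; FindNextTargetLocation stores the destination returned by its TargetLocator, and DoObjective has its ObjectiveExecuter attempt the objective at the target location.
; Getters expose that destination, plus the flying flag and movement speed multiplier read from SpeciesData, keeping species traits data-driven.
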(event EventDoObjective
  (Default|AttemptObjectiveatTargetLocation (Variables|Default|GetobjectiveExecuter)))

(event EventFindNextTargetLocation
  (bind _location (Default|FindParentAnimalNextTargetLocation (Variables|Default|GettargetLocator)))
  (Variables|Default|SetnextTargetLocation _location))

(event EventBeginPlay
  (bind _asaic_animal (Utilities|Casting|CastToAIC_animal (AI|GetAIController self)))
  (Variables|Default|SetanimalController _asaic_animal))

(fn ConstructionScript)

(fn GetIsFlying
  (return (.isflying (Variables|Default|GetspeciesData))))

(fn GetMovementMultiplier
  (return (.movementspeedmultiplier (Variables|Default|GetspeciesData))))

(fn GetNextTargetLocation
  (return (Variables|Default|GetnextTargetLocation)))