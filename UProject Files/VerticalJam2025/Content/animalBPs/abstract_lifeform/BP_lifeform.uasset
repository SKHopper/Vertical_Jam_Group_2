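; BP_lifeform is a base lifeform character Blueprint that configures itself from its SpeciesData.
; On BeginPlay, SetupSelf scales the CharacterMovement max walk speed by the species multiplier.
; SetupComponents then adds each component class listed in SpeciesData at runtime, passing the lifeform as ParentAnimal, so species are composed from data.
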(event EventBeginPlay
  (CallFunction|SetupSelf)
  (CallFunction|SetupComponents))

(fn ConstructionScript)

(fn SetupComponents
  (for _array_element (.components (Utilities|Struct|BreakF_animalSpecies (Variables|Default|GetspeciesData)))
    (Game|AddComponentbyClass _array_element self)))

(fn SetupSelf
  (bind _charactermovement (Variables|Character|GetCharacterMovement))
  (Variables|/Script/Engine.CharacterMovementComponent|SetMaxWalkSpeed _charactermovement (* (Variables|/Script/Engine.CharacterMovementComponent|GetMaxWalkSpeed _charactermovement) (.movementSpeedMultiplier (Utilities|Struct|BreakF_animalSpecies (Variables|Default|GetspeciesData))))))