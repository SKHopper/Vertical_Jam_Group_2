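; AC_attackBees is an animal behaviour component that makes its parent animal, bees by name, chase and attack the player.
; Its target search returns the player's location within SightRange, keeping the animal's own height unless its species flies, and otherwise uses the parent class's result.
; When attempting its objective at the target, it sends AttackMessage to the player if within AttackRange.
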(event EventAttemptObjectiveatTargetLocation
  (if (<= (Math|Vector|Distance(Vector) (Transformation|GetActorLocation (Game|GetPlayerCharacter 0)) (Transformation|GetActorLocation (Variables|Default|GetparentAnimal))) (Variables|Default|GetattackRange))
    (Class|AttackIF|Attack(Message) (Game|GetPlayerCharacter 0))))

(fn FindParentAnimalNextTargetLocation
  (bind _returnvalue (Game|GetPlayerCharacter 0))
  (bind _parentanimal (Variables|Default|GetparentAnimal))
  (bind _returnvalue_2 (Transformation|GetActorLocation _returnvalue))
  (bind _returnvalue_3 (Transformation|GetActorLocation _parentanimal))
  (bind _location (|CallParentFunction))
  (return (Math|Vector|SelectVector _location (Math|Vector|MakeVector (.x _returnvalue_2) (.y _returnvalue_2) (Math|Float|SelectFloat (.z _returnvalue_2) (.z _returnvalue_3) (.isFlying (Utilities|Struct|BreakF_animalSpecies (Variables|/Game/animalBPs/abstract_lifeform/BP_lifeform.BP_lifeform_C|GetspeciesData _parentanimal))))) (> (Math|Vector|Distance(Vector) (Math|Vector|MakeVector (.x _returnvalue_2) (.y _returnvalue_2) (.z _returnvalue_2)) (Math|Vector|MakeVector (.x _returnvalue_3) (.y _returnvalue_3) (.z _returnvalue_3))) (Variables|Default|GetsightRange)))))