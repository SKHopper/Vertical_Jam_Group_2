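; Animal behaviour component that makes its parent animal seek out and attack hornet lifeforms.
; Target selection scans all BP_lifeform actors for the nearest hornet within sight range, with a helper graph referencing the "Norfolk Hawker" display name.
; The target's position overrides the parent movement destination, matching height only for flying species.
; At the destination, it sends AttackMessage if the target is within attack range scaled by species interaction scale.
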(event EventAttemptObjectiveatTargetLocation
  (bind _parentanimal (Variables|Default|GetparentAnimal))
  (bind _target (Variables|Default|Gettarget))
  (Utilities|IsValid _target
    (:Is%20Valid
      (if (<= (Math|Vector|Distance(Vector) (Transformation|GetActorLocation _target) (Transformation|GetActorLocation _parentanimal)) (* (Variables|Default|GetattackRange) (.interactionscale (Variables|/Game/animalBPs/abstract_lifeform/BP_lifeform.BP_lifeform_C|GetspeciesData _parentanimal))))
        (Class|AttackIF|Attack(Message) (Variables|Default|Gettarget))))))

(fn FindParentAnimalNextTargetLocation
  (bind _parentanimal (Variables|Default|GetparentAnimal))
  (bind _target (Variables|Default|Gettarget))
  (bind _returnvalue (Transformation|GetActorLocation _target))
  (bind _location (|CallParentFunction))
  (CallFunction|SelectTarget)
  (Utilities|IsValid _target
    (:Is%20Valid
      (return (Math|Vector|MakeVector (.x _returnvalue) (.y _returnvalue) (Math|Float|SelectFloat (.z _returnvalue) (.z (Transformation|GetActorLocation _parentanimal)) (.isFlying (Utilities|Struct|BreakF_animalSpecies (Variables|/Game/animalBPs/abstract_lifeform/BP_lifeform.BP_lifeform_C|GetspeciesData _parentanimal)))))))
    (:Is%20Not%20Valid
      (return _location))))

(fn SelectTarget
  (bind _outactors (Actor|GetAllActorsOfClass "/Game/animalBPs/abstract_lifeform/BP_lifeform.BP_lifeform_C"))
  (for _array_element _outactors
    (if (Utilities|IsLifeformHornet _array_element)
      (if (and (< (Utilities|Distance _array_element) (LocalVariables|GetsmallestDistance)) (<= (Utilities|Distance _array_element) (Variables|Default|GetsightRange)))
        (LocalVariables|SetsmallestDistance (Utilities|Distance _array_element))
        (Variables|Default|Settarget _array_element)))))