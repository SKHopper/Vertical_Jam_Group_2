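; Animal behavior component that makes its parent animal seek out and attack plants.
; Target-location lookup scans all BP_plant actors for one nearer than SmallestDistance, which this graph never resets, and stores it as Target.
; It returns the plant's position, using plant height only for flying species, or falls back to the parent implementation without a valid Target.
; The objective attempt sends AttackMessage to the Target when within AttackRange.
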(event EventAttemptObjectiveatTargetLocation
  (bind _target (Variables|Default|Gettarget))
  (Utilities|IsValid _target
    (:Is%20Valid
      (if (<= (Math|Vector|Distance(Vector) (Transformation|GetActorLocation _target) (Transformation|GetActorLocation (Variables|Default|GetparentAnimal))) (Variables|Default|GetattackRange))
        (Class|AttackIF|Attack(Message) (Variables|Default|Gettarget))))))

(fn FindParentAnimalNextTargetLocation
  (bind _parentanimal (Variables|Default|GetparentAnimal))
  (bind _target (Variables|Default|Gettarget))
  (bind _returnvalue (Transformation|GetActorLocation _target))
  (bind _location (|CallParentFunction))
  (CallFunction|SelectTargetPlant)
  (Utilities|IsValid _target
    (:Is%20Valid
      (return (Math|Vector|MakeVector (.x _returnvalue) (.y _returnvalue) (Math|Float|SelectFloat (.z _returnvalue) (.z (Transformation|GetActorLocation _parentanimal)) (.isFlying (Utilities|Struct|BreakF_animalSpecies (Variables|/Game/animalBPs/abstract_lifeform/BP_lifeform.BP_lifeform_C|GetspeciesData _parentanimal)))))))
    (:Is%20Not%20Valid
      (return _location))))

(fn SelectTargetPlant
  (bind _outactors (Actor|GetAllActorsOfClass "/Game/plant/BP_plant.BP_plant_C"))
  (for _array_element _outactors
    (if (< (Math|Vector|Distance(Vector) (Transformation|GetActorLocation _array_element) (Transformation|GetActorLocation (Variables|Default|GetparentAnimal))) (LocalVariables|GetsmallestDistance))
      (LocalVariables|SetsmallestDistance (Math|Vector|Distance(Vector) (Transformation|GetActorLocation _array_element) (Transformation|GetActorLocation (Variables|Default|GetparentAnimal))))
      (Variables|Default|Settarget _array_element))))