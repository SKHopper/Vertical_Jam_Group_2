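; Animal behaviour component that acts as both objective executer and target locator for its parent animal.
; On BeginPlay it registers itself in both roles and starts the move loop on the animal's AI controller.
; Its next-target function calls the parent version, then returns GetRandomRoamLocation.
; That roam function holds only an unconnected random-offset calculation around the animal's position.
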(event EventBeginPlay
  (bind _self self)
  (bind _parentanimal (Variables|Default|GetparentAnimal))
  (Variables|/Game/animalBPs/abstract_lifeform/BP_lifeform.BP_lifeform_C|SetobjectiveExecuter _parentanimal _self)
  (Variables|/Game/animalBPs/abstract_lifeform/BP_lifeform.BP_lifeform_C|SettargetLocator _parentanimal _self)
  (bind _asaic_animal (Utilities|Casting|CastToAIC_animal (AI|GetAIController _parentanimal)))
  (Default|BeginAIMoveLoop _asaic_animal))

(fn FindParentAnimalNextTargetLocation
  (|CallParentFunction)
  (return (Utilities|GetRandomRoamLocation)))