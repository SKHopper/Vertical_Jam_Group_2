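; Animal behaviour component that scares nearby Green Woodpeckers away when its animal attempts its objective at a target location.
; It scans every BP_animal actor for woodpeckers, identified by species display name, within SightRange.
; Each match's AnimalController is force-moved a fixed distance directly away from the owner.
; Choosing the next target location is left to the parent behaviour class.
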(event EventAttemptObjectiveatTargetLocation
  (CallFunction|ScareWoodpeckers))

(fn FindParentAnimalNextTargetLocation
  (bind _location (|CallParentFunction))
  (return _location))

(fn ScareWoodpeckers
  (bind _outactors (Actor|GetAllActorsOfClass "/Game/animalBPs/BP_animal_.BP_animal__C"))
  (for _array_element _outactors
    (if (and (Utilities|IsLifeformWoodPecker _array_element) (<= (Utilities|Distance _array_element) (Variables|Default|GetsightRange)))
      (LocalVariables|SetsmallestDistance (Utilities|Distance _array_element))
      (Default|ForceMove (Variables|/Game/animalBPs/BP_animal_.BP_animal__C|GetanimalController _array_element) (+ (* (Math|Vector|GetUnitDirection(Vector) (Transformation|GetActorLocation (Components|GetOwner)) (Transformation|GetActorLocation _array_element)) 5e+02) (Transformation|GetActorLocation _array_element))))))