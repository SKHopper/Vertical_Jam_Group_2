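; Beehive actor that serves as player spawn, nectar store and honey bank, registering itself with GS_main.
; Interacting deposits the player's nectar and sets the hive's Z scale from honey versus the win threshold.
; A looping timer converts nectar to honey and updates the honey bar widget.
; Attacks drain honey, while respawns spend it or trigger GameState's Lose when honey is short.
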(event Custom|respawnPlayer
  (CallFunction|TryRespawn))

(event EventBeginPlay
  (CallFunction|SetupGameState)
  (CallFunction|SetupPlayer)
  (CallFunction|NectarConversionLoop)
  (bind _asuw_honey_bar (Utilities|Casting|CastToUW_honeyBar (UserInterface|GetWidget (Variables|Default|Getbar))))
  (Variables|Default|SetAs%20UW%20Honey%20Bar _asuw_honey_bar)
  (Variables|/Game/beehive/UW_honeyBar.UW_honeyBar_C|Setmax _asuw_honey_bar (Variables|/Game/main_level/GS_main.GS_main_C|GethoneyWinThreshold (Variables|Default|GetgameState))))

(event EventAttack
  (Variables|Default|Sethoney (Math|Float|Clamp(Float) (- (Variables|Default|Gethoney) 1.0) 0.0 999999.0)))

(event EventInteract
  (CallFunction|NectarDeposit)
  (Transformation|SetRelativeScale3D (Variables|Default|GetScene) (Math|Vector|MakeVector 1.0 1.0 (/ (Variables|Default|Gethoney) (Variables|/Game/main_level/GS_main.GS_main_C|GethoneyWinThreshold (Variables|Default|GetgameState))))))

(fn ConstructionScript)

(fn NectarDeposit
  (bind _nectar (Default|DepositNectar (Variables|Default|Getplayer)))
  (Variables|Default|Setnectar (+ _nectar (Variables|Default|Getnectar)))
  (Audio|PlaySound2D "/Game/audio/other/bubble-pop-06-351337.bubble-pop-06-351337" 1.0 1.0 0.0 0 0))

(fn SetupPlayer
  (bind _asbp_top_down_character (Utilities|Casting|CastToBP_TopDownCharacter (Game|GetPlayerCharacter 0)))
  (bind _output_get (Variables|Default|Setplayer _asbp_top_down_character))
  (Transformation|SetActorLocation _output_get (Transformation|GetWorldLocation (Variables|Default|GetplayerSpawnPoint)) false false))

(fn ConvertNectartoHoney
  (if (>= (Variables|Default|Getnectar) 1.0)
    (Math|Float|DecrementFloat (Variables|Default|Getnectar)
      (:%20%20
        (bind _output_get (Variables|Default|Sethoney (+ (Variables|Default|Gethoney) (Variables|Default|GethoneyPerNectar))))
        (Default|Set (Variables|Default|GetAs%20UW%20Honey%20Bar) _output_get)))))

(fn NectarConversionLoop
  (bind _returnvalue (Utilities|Time|SetTimerbyFunctionName 0 "convertNectarToHoney" (Variables|Default|GettimeToConvertNectar) true))
  (Variables|Default|SetnectarConversionTimer _returnvalue))

(fn SetupGameState
  (bind _asgs_main (Utilities|Casting|CastToGS_main (Game|GetGameState)))
  (bind _output_get (Variables|Default|SetgameState _asgs_main))
  (Variables|/Game/main_level/GS_main.GS_main_C|Setbeehive _output_get self))

(fn TryRespawn
  (if (> (Variables|Default|GetrespawnCost) (Variables|Default|Gethoney))
    (Default|Lose (Variables|Default|GetgameState) true)
    (else
      (bind _output_get (Variables|Default|Sethoney (- (Variables|Default|Gethoney) (Variables|Default|GetrespawnCost))))
      (Default|RespawnEffect (Variables|Default|Getplayer))
      (Default|Set (Variables|Default|GetAs%20UW%20Honey%20Bar) _output_get))))

(fn DepositNectar
  (return 0.0))