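; Plant actor that grows through Sapling, Stem and Flowering stages, with meshes, transforms and extra components supplied by SpeciesData.
; Looping timers ease each part's scale, and a full-grown flower creates a pollen aura via BPAuraManagerComponent.
; Pollination launches seeds, then kills annuals or drops the flower to regrow.
; Attacks topple the current stage and set growth back or kill saplings; death also follows a timer, sinking the plant before destruction.
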(event Custom|die
  (bind _defaultsceneroot (Variables|Default|GetDefaultSceneRoot))
  (bind _pollen_cloud (Variables|Default|Getpollen%20cloud))
  ;[0.15 0.15 0.15 0.5] plant down anim
  (Rendering|Material|SetMaterial (Variables|Default|GetgroundLeaves) 0 "/Game/Levels/Materials/M_Brick_Clay_New1.M_Brick_Clay_New1")
  (for _array_element (Variables|/Game/pollen_collect/Pollen/BP_PollenAura.BP_PollenAura_C|GetOwnOrbs _pollen_cloud)
    (Actor|DestroyActor _array_element))
  (Actor|DestroyActor _pollen_cloud)
  (Utilities|FallinRandomDirection _defaultsceneroot 0.0)
  (Rendering|Material|SetMaterial (Variables|Default|Getstem) 0 "/Game/Levels/Materials/M_Brick_Clay_New1.M_Brick_Clay_New1")
  (Components|MoveComponentTo _defaultsceneroot (- (Variables|/Script/Engine.SceneComponent|GetRelativeLocation _defaultsceneroot) "0.000000,0.000000,1000.000000") (Variables|/Script/Engine.SceneComponent|GetRelativeRotation _defaultsceneroot) false true 1e+01 false)
  (Actor|DestroyActor))

(event Custom|queueDeath
  (bind _returnvalue (Utilities|Time|SetTimerbyEvent (delegate Custom|die) (Utilities|GetDeathTime)))
  (Variables|Default|SetdeathTImer _returnvalue))

(event Custom|reset%20stem
  (bind _stem (Variables|Default|Getstem))
  ;[0.15 0.15 0.15 0.5] take damage
  (Utilities|FallinRandomDirection _stem 1e+04)
  (Transformation|SetRelativeScale3D _stem "0, 0, 0")
  (Variables|Default|Setgrew%20stem false))

(event Custom|able%20to%20make%20seeds
  (bind _speciesdata (Variables|Default|GetspeciesData))
  (Utilities|FlowControl|DoOnce true) ; enters at Reset
)

(event Custom|grow
  (switch Utilities|FlowControl|Switch|SwitchonE_plantStage (Variables|Default|GetgrowthStage)
    (:NewEnumerator0
      (Variables|Default|SetgrowthStage "NewEnumerator1")
      (CallFunction|GrowStem)
      (bind _returnvalue (Utilities|Time|SetTimerbyEvent (delegate Custom|grow) (stale EventBeginPlay _output_get)))
      (Variables|Default|SetgrowthTimer _returnvalue))
    (:NewEnumerator1
      (Variables|Default|SetgrowthStage "NewEnumerator2")
      (CallFunction|GrowFlower)
      (bind _returnvalue_2 (Utilities|Time|SetTimerbyEvent (delegate Custom|die) (Utilities|GetDeathTime)))
      (Variables|Default|SetdeathTImer _returnvalue_2))))

(event Custom|growStem
  (if (Utilities|Enum|Equal(Enum) (Variables|Default|GetgrowthStage) "NewEnumerator1")
    ;[0.15 0.15 0.15 0.5] stem upward anim
    (Rendering|SetVisibility (Variables|Default|Getstem) true false)
    (Utilities|Time|SetTimerbyEvent (delegate Custom|increment%20stem%20size) 0.05)))

(event Custom|growFlower
  ;[0.15 0.15 0.15 0.5] flower outward anim
  (if (and (Variables|Default|Getgrew%20stem) (Utilities|Enum|Equal(Enum) (Variables|Default|GetgrowthStage) "NewEnumerator2"))
    (Rendering|SetVisibility (Variables|Default|Getflower) true false)
    (Utilities|Time|SetTimerbyEvent (delegate Custom|increment%20flower%20size) 0.05)
    (else
      ;[0.15 0.15 0.15 0.5] queue pollen creation
      (Variables|Default|SetgrowthStage "NewEnumerator0")
      (CallFunction|Grow))))

(event Custom|growGroundLeaves
  ;[0.15 0.15 0.15 0.5] groundLeaves up anim
  (Rendering|SetVisibility (Variables|Default|GetgroundLeaves) true false)
  (Utilities|Time|SetTimerbyEvent (delegate Custom|increment%20ground%20leaf%20size) 0.05))

(event Custom|increment%20ground%20leaf%20size
  ;[0.15 0.15 0.15 0.5] groundLeaves up anim
  (Utilities|EaseScaleTowardTarget (Variables|Default|GetgroundLeaves) (.Scale (Math|Transform|BreakTransform (.groundleaffinalrelativetransform (Variables|Default|GetspeciesData))))
    (:loop
      (Utilities|Time|SetTimerbyEvent (delegate Custom|increment%20ground%20leaf%20size) 0.05))))

(event Custom|increment%20stem%20size
  ;[0.15 0.15 0.15 0.5] stem upward anim
  (Utilities|EaseScaleTowardTarget (Variables|Default|Getstem) (.Scale (Math|Transform|BreakTransform (.stemfinalrelativetransform (Variables|Default|GetspeciesData))))
    (:loop
      (if (Utilities|Enum|Equal(Enum) (Variables|Default|GetgrowthStage) "NewEnumerator1")
        (Utilities|Time|SetTimerbyEvent (delegate Custom|increment%20stem%20size) 0.05)
        (elif (not (Utilities|Enum|Equal(Enum) (Variables|Default|GetgrowthStage) "NewEnumerator2"))
          (CallFunction|ResetFlower)
          (Variables|Default|SetgrowthStage "NewEnumerator0")
          (CallFunction|Grow))))
    (:done
      (Variables|Default|Setgrew%20stem true)
      (CallFunction|Grow))))

(event Custom|increment%20flower%20size
  (bind _speciesdata (Variables|Default|GetspeciesData))
  ;[0.15 0.15 0.15 0.5] flower outward anim
  (Utilities|EaseScaleTowardTarget (Variables|Default|Getflower) (.Scale (Math|Transform|BreakTransform (.flowerfinalrelativetransform _speciesdata)))
    (:loop
      (if (Utilities|Enum|Equal(Enum) (Variables|Default|GetgrowthStage) "NewEnumerator2")
        (Utilities|Time|SetTimerbyEvent (delegate Custom|increment%20flower%20size) 0.05)
        (else
          (CallFunction|ResetFlower)
          ;[0.15 0.15 0.15 0.5] queue pollen creation
          (Variables|Default|SetgrowthStage "NewEnumerator0" :!label _label)
          (CallFunction|Grow))))
    (:done
      (Utilities|FlowControl|DelayUntilNextTick)
      (if (Utilities|Enum|Equal(Enum) (Variables|Default|GetgrowthStage) "NewEnumerator2")
        (bind _spawned_auras (Default|ConstructAura (Variables|Default|GetBP_AuraManager_Component) self (+ (Transformation|GetWorldLocation (Variables|Default|Getflower)) (.pollenauraoffset _speciesdata)) (Variables|Default|GetspeciesData) self))
        (Variables|Default|Setpollen%20cloud _spawned_auras)
        (Components|Activation|Activate (Variables|Default|GetN_Nectar) false)
        (CallFunction|AbletoMakeSeeds)
        (else
          (goto _label))))))

(event Custom|reset%20flower
  (bind _pollen_cloud (Variables|Default|Getpollen%20cloud))
  (bind _flower (Variables|Default|Getflower))
  ;[0.15 0.15 0.15 0.5] take damage
  (for _array_element (Variables|/Game/pollen_collect/Pollen/BP_PollenAura.BP_PollenAura_C|GetOwnOrbs _pollen_cloud)
    (Actor|DestroyActor _array_element))
  (Actor|DestroyActor _pollen_cloud)
  (Utilities|FallinRandomDirection _flower 1e+04)
  (Transformation|SetRelativeScale3D _flower "0, 0, 0"))

(event EventPollinated
  (bind _speciesdata (Variables|Default|GetspeciesData))
  (Utilities|FlowControl|DoOnce true
    (:Completed
      ;[0.15 0.15 0.15 0.5] make seed(s)
      (for _index (range 1 (.seedsspawnperpollinate _speciesdata))
        (bind _returnvalue (Game|SpawnActorfromClass :Class "/Game/seed_test/BP_Master_Seed.BP_Master_Seed_C" :SpawnTransform (Transformation|GetWorldTransform (Variables|Default|Getflower)) :CollisionHandlingOverride "Undefined" :TransformScaleMethod "MultiplyWithRoot" :Instigator 0))
        (Variables|/Game/seed_test/BP_Master_Seed.BP_Master_Seed_C|SetSpecies%20Data _returnvalue (Variables|Default|GetspeciesData))
        (Physics|SetPhysicsLinearVelocity (Variables|/Game/seed_test/BP_Master_Seed.BP_Master_Seed_C|GetSeed _returnvalue) (* (Math|Random|RandomUnitVectorinConeinDegrees "0.000000,0.000000,1.000000" 3e+01) 1e+03) false "None"))
      (Utilities|FlowControl|Delay 2.0)
      (if (.isanualplantdiesaftermakingseeds _speciesdata)
        (CallFunction|Die)
        (else
          ;[0.15 0.15 0.15 0.5] take damage
          ;;[0.15 0.15 0.15 0.5] drop flower
          (Variables|Default|SetgrowthStage "NewEnumerator1")
          (CallFunction|ResetFlower)
          (Utilities|FlowControl|Delay 1.1)
          (CallFunction|PositionParts)
          (CallFunction|Grow))))))

(event EventKill
  (bind _defaultsceneroot (Variables|Default|GetDefaultSceneRoot))
  (bind _pollen_cloud (Variables|Default|Getpollen%20cloud))
  ;[0.15 0.15 0.15 0.5] plant down anim
  (Rendering|Material|SetMaterial (Variables|Default|GetgroundLeaves) 0 "/Game/Levels/Materials/M_Brick_Clay_New1.M_Brick_Clay_New1")
  (for _array_element (Variables|/Game/pollen_collect/Pollen/BP_PollenAura.BP_PollenAura_C|GetOwnOrbs _pollen_cloud)
    (Actor|DestroyActor _array_element))
  (Actor|DestroyActor _pollen_cloud)
  (Utilities|FallinRandomDirection _defaultsceneroot 0.0)
  (Rendering|Material|SetMaterial (Variables|Default|Getstem) 0 "/Game/Levels/Materials/M_Brick_Clay_New1.M_Brick_Clay_New1")
  (Components|MoveComponentTo _defaultsceneroot (- (Variables|/Script/Engine.SceneComponent|GetRelativeLocation _defaultsceneroot) "0.000000,0.000000,1000.000000") (Variables|/Script/Engine.SceneComponent|GetRelativeRotation _defaultsceneroot) false true 1e+01 false)
  (Actor|DestroyActor))

(event EventBeginPlay
  (CallFunction|PositionParts)
  (CallFunction|MakeComponents)
  (CallFunction|GrowGroundLeaves)
  (bind _output_get (Variables|Default|SetgrowIndividualStageTime (Utilities|GetGrowthIndividualStageTime)))
  (bind _returnvalue (Utilities|Time|SetTimerbyEvent (delegate Custom|grow) _output_get))
  (Variables|Default|SetgrowthTimer _returnvalue))

(event EventAttack
  (bind _defaultsceneroot (Variables|Default|GetDefaultSceneRoot))
  ;[0.15 0.15 0.15 0.5] take damage
  (switch Utilities|FlowControl|Switch|SwitchonE_plantStage (Variables|Default|GetgrowthStage)
    (:NewEnumerator0
      ;[0.15 0.15 0.15 0.5] plant down anim
      (Utilities|FallinRandomDirection _defaultsceneroot 0.0)
      (Rendering|Material|SetMaterial (Variables|Default|Getstem) 0 "/Game/Levels/Materials/M_Brick_Clay_New1.M_Brick_Clay_New1")
      (Components|MoveComponentTo _defaultsceneroot (- (Variables|/Script/Engine.SceneComponent|GetRelativeLocation _defaultsceneroot) "0.000000,0.000000,1000.000000") (Variables|/Script/Engine.SceneComponent|GetRelativeRotation _defaultsceneroot) false true 1e+01 false)
      (Actor|DestroyActor))
    (:NewEnumerator1
      ;;[0.15 0.15 0.15 0.5] drop stem
      (Variables|Default|SetgrowthStage "NewEnumerator0")
      (CallFunction|ResetFlower)
      (CallFunction|ResetStem)
      (Utilities|FlowControl|Delay 1.1)
      (CallFunction|PositionParts)
      (CallFunction|Grow))
    (:NewEnumerator2
      ;;[0.15 0.15 0.15 0.5] drop flower
      (Variables|Default|SetgrowthStage "NewEnumerator1")
      (CallFunction|ResetFlower)
      (Utilities|FlowControl|Delay 1.1)
      (CallFunction|PositionParts)
      (CallFunction|Grow))))

(fn ConstructionScript)

(fn MakeComponents
  (for _array_element (.plantComponents (Utilities|Struct|BreakF_plantSpecies (Variables|Default|GetspeciesData)))
    (Game|AddComponentbyClass _array_element)))

(fn PositionParts
  (bind _stem (Variables|Default|Getstem))
  (bind _flower (Variables|Default|Getflower))
  (bind _speciesdata (Variables|Default|GetspeciesData))
  (bind _groundleaves (Variables|Default|GetgroundLeaves))
  (bind (_location _rotation) (Math|Transform|BreakTransform (.flowerfinalrelativetransform _speciesdata)))
  (bind (_location_2 _rotation_2) (Math|Transform|BreakTransform (.groundleaffinalrelativetransform _speciesdata)))
  (bind (_location_3 _rotation_3) (Math|Transform|BreakTransform (.stemfinalrelativetransform _speciesdata)))
  (Utilities|FlowControl|Sequence
    (:then_0
      (Transformation|SetRelativeLocationAndRotation _groundleaves _location_2 _rotation_2 false false)
      (Components|StaticMesh|SetStaticMesh _groundleaves (.groundleafmesh _speciesdata)))
    (:then_1
      (Transformation|SetRelativeLocationAndRotation _stem _location_3 _rotation_3 false false)
      (Components|StaticMesh|SetStaticMesh _stem (.stemmesh _speciesdata)))
    (:then_2
      (Transformation|SetRelativeLocationAndRotation _flower _location _rotation false false)
      (Components|StaticMesh|SetStaticMesh _flower (.flowermesh _speciesdata)))))