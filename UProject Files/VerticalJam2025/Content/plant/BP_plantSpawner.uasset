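; Plant spawner actor that randomly populates a set of spawn points with BP_plant actors at game start.
; On BeginPlay it reads all species rows from a data table and sums their relative spawn weights.
; Each spawn point rolls a spawn chance, picks a species by cumulative weighted random selection, then spawns a plant with that species data and a random yaw.
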(event EventBeginPlay
  (bind _outrownames (DataTable|GetDataTableRowNames (Variables|Default|GetspeciesDataTable)))
  (bind _output_get (Variables|Default|SetspeciesIDs _outrownames))
  (for _array_element _output_get
    (bind _returnvalue (Utilities|GetDataTableRow (Variables|Default|GetspeciesDataTable) _array_element)
      (:then
        (Variables|Default|SetspawnWeightTotal (+ (.spawnWeightRelative (Utilities|Struct|BreakF_plantSpecies _returnvalue)) (Variables|Default|GetspawnWeightTotal))))))
  (CallFunction|SpawnPlants))

(fn ConstructionScript)

(fn SpawnPlants
  (for _array_element (Variables|Default|GetspawnPoints)
    (if (Math|Random|RandomBoolwithWeight (Variables|Default|GetchanceSpawnPlant))
      (LocalVariables|SetspawnWeightSelector (Math|Random|RandomIntegerinRange 0 (Variables|Default|GetspawnWeightTotal)))
      (LocalVariables|SetweightsTracker 0)
      (bind _array_element_2 (Utilities|Array|ForEachLoopwithBreak (Variables|Default|GetspeciesIDs) :!label _label)
        (:LoopBody
          (bind _returnvalue (Utilities|GetDataTableRow (Variables|Default|GetspeciesDataTable) _array_element_2)
            (:then
              (bind _output_get (LocalVariables|SetweightsTracker (+ (.spawnWeightRelative (Utilities|Struct|BreakF_plantSpecies _returnvalue)) (LocalVariables|GetweightsTracker))))
              (if (>= _output_get (LocalVariables|GetspawnWeightSelector))
                (LocalVariables|SetspeciesData _returnvalue)
                (goto _label Break)))))
        (:Completed
          (Game|SpawnActorfromClass "/Game/plant/BP_plant.BP_plant_C" (Math|Transform|MakeTransform (Transformation|GetActorLocation _array_element) (Math|Rotator|MakeRotator 0.0 0.0 (Math|Random|RandomFloatinRange 0.0 359.9)) "1.000000,1.000000,1.000000") "Undefined" "MultiplyWithRoot" 0 (LocalVariables|GetspeciesData) 0))))))