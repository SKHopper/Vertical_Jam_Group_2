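; Plant property component that gives its owning BP_plant a shading effect, suppressing younger plants growing nearby.
; After one growth-stage delay, it attaches a dark-tinted local fog volume to the plant's stem as the visible shade.
; It then runs a sphere overlap, repeated on a looping timer, with radius scaled by stem height scale, killing other plants still in early growth stages.
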(event Custom|kill%20competitors
  (bind _outactors (Collision|SphereOverlapActors (Transformation|GetActorLocation (stale EventBeginPlay _asbp_plant)) (* (.z (Transformation|GetActorScale3D (Variables|/Game/plant/BP_plant.BP_plant_C|Getstem%20actor (stale EventBeginPlay _asbp_plant)))) 6e+02) (Variables|Default|GetObject%20Types) "/Game/plant/BP_plant.BP_plant_C" (Utilities|Array|MakeArray (stale EventBeginPlay _asbp_plant))))
  (for _array_element _outactors
    (bind _asbp_plant (Utilities|Casting|CastToBP_plant _array_element))
    (if (< (Variables|/Game/plant/BP_plant.BP_plant_C|GetgrowthStage _asbp_plant) 3)
      (Default|Die _asbp_plant))))

(event EventBeginPlay
  (bind _asbp_plant (Utilities|Casting|CastToBP_plant (Components|GetOwner)))
  (Utilities|FlowControl|Delay (Variables|/Game/plant/BP_plant.BP_plant_C|GetgrowIndividualStageTime _asbp_plant))
  (bind _returnvalue (Game|AddComponentbyClass _asbp_plant "/Script/Engine.LocalFogVolumeComponent" false))
  (Transformation|AttachComponentToComponent _returnvalue (Variables|/Script/Engine.Actor|GetRootComponent (Variables|/Game/plant/BP_plant.BP_plant_C|Getstem%20actor _asbp_plant)) "None" "KeepWorld" "KeepRelative" "KeepRelative" true)
  (Class|LocalFogVolumeComponent|SetFogAlbedo _returnvalue "(R=0.006466,G=0.000000,B=0.088542,A=1.000000)")
  (Class|LocalFogVolumeComponent|SetHeightFogFalloff _returnvalue 1e+02)
  (Utilities|Time|SetTimerbyEvent (delegate Custom|kill%20competitors) 5.0 true)
  (bind _outactors (Collision|SphereOverlapActors (Transformation|GetActorLocation _asbp_plant) (* (.z (Transformation|GetActorScale3D (Variables|/Game/plant/BP_plant.BP_plant_C|Getstem%20actor _asbp_plant))) 6e+02) (Variables|Default|GetObject%20Types) "/Game/plant/BP_plant.BP_plant_C" (Utilities|Array|MakeArray _asbp_plant)))
  (for _array_element _outactors
    (bind _asbp_plant_2 (Utilities|Casting|CastToBP_plant _array_element))
    (if (< (Variables|/Game/plant/BP_plant.BP_plant_C|GetgrowthStage _asbp_plant_2) 3)
      (Default|Die _asbp_plant_2))))