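; Base pollen orb with colored trail that can roam within its parent aura and homes in on the player for collection.
; While the player is in radius, a gated Tick rebuilds InterpToMovement points toward a jittered player position, scaling duration by distance until a short timer forces near-instant travel.
; Player overlap spawns a color-matched collect actor, notifies the aura, adds nectar and pollen through BP_ResourceManager, then destroys the orb.
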(event OnComponentBeginOverlap(Collision)
  (params (OverlappedComponent :type Primitive%20Component%20Object%20Reference) (OtherActor :type Actor%20Object%20Reference) (OtherComp :type Primitive%20Component%20Object%20Reference) (OtherBodyIndex :type Integer) (bFromSweep :type Boolean) (SweepResult :type Hit%20Result%20Structure%20%28by%20ref%29))
  ;[0.1484 0.375 0.0293 0.5] Collect on Overlap
  (if (== OtherActor (Game|GetPlayerCharacter 0))
    (bind _returnvalue (Game|SpawnActorfromClass "/Game/pollen_collect/Pollen/BP_PollenCollect.BP_PollenCollect_C" (Transformation|GetWorldTransform (Variables|Default|GetPollen)) "AlwaysSpawn" "MultiplyWithRoot" 0 0))
    (bind (_colormin _colormax) (CallFunction|GetMaterialColors))
    (Default|SetupColor _returnvalue _colormin _colormax)
    (Default|PollenPickup (Variables|Default|GetParentAura) self)
    (CallFunction|ResourceIncrease)
    (Actor|DestroyActor)))

(event Custom|InstantCollect
  ;[0.7292 0.03726 0 0.5] Event is tied to the timer function above
  (Variables|/Script/Engine.InterpToMovementComponent|SetDuration (Variables|Default|GetInterpToMovement) (Math|Random|RandomFloatinRange 0.0 0.05))
  (Variables|Default|SetInstantTimerElapsed true))

(event EventBeginPlay)

(event EventBeeinRadius
  ;[0.07275 0.1502 0.776 0.5] Is triggered when the player enters the Parent Aura's Boundry
  (Utilities|Time|SetTimerbyFunctionName 0 "InstantCollect" 0.2)
  (Variables|/Script/Engine.InterpToMovementComponent|SetBehaviourType (Variables|Default|GetInterpToMovement) "OneShot")
  (Utilities|FlowControl|Gate true) ; enters at Open
)

(event EventTick
  (params (DeltaSeconds :type Float%20%28single-precision%29))
  ;[0.07275 0.1502 0.776 0.5] Is triggered when the player enters the Parent Aura's Boundry
  (Utilities|FlowControl|Gate true
    (:Exit
      (if (not (Utilities|Operators|EqualEqual :A (Transformation|GetActorLocation (Game|GetPlayerCharacter 0))))
        (CallFunction|NodesGotoPlayer)
        (Class|InterptoMovementComponent|RestartMovement (Variables|Default|GetInterpToMovement) 1.0)))))

(event EventBeeLeaveRadius
  ;[0.07275 0.1502 0.776 0.5] Is triggered when the player enters the Parent Aura's Boundry
  (Utilities|FlowControl|Gate true) ; enters at Close
)

(fn ConstructionScript
  (bind _returnvalue (Rendering|Material|CreateDynamicMaterialInstance (Rendering|Material|GetMaterial (Variables|Default|GetPollen) 0) "OrbMat" "None" :!class /Script/Engine.KismetMaterialLibrary))
  (bind _output_get (Variables|Default|SetOrb_Material _returnvalue))
  (Rendering|Material|SetMaterial (Variables|Default|GetPollen) 0 _output_get))

(fn NodesGotoPlayer
  (bind _returnvalue (Game|GetPlayerCharacter 0))
  (bind _returnvalue_2 (Game|GetPlayerCharacter 0))
  (bind _interptomovement (Variables|Default|GetInterpToMovement))
  (bind _pollen (Variables|Default|GetPollen))
  (bind _interptomovement_2 (Variables|Default|GetInterpToMovement))
  (bind _returnvalue_3 (Transformation|GetWorldLocation _pollen))
  (bind _returnvalue_4 (Transformation|GetActorLocation _returnvalue))
  (bind _returnvalue_5 (Transformation|GetActorLocation _returnvalue_2))
  (bind _returnvalue_6 (Math|Vector|Distance(Vector) _returnvalue_3 _returnvalue_4))
  (bind _returnvalue_7 (/ _returnvalue_6 1.15e+03))
  (Class|InterptoMovementComponent|ResetControlPoints _interptomovement)
  (Class|InterptoMovementComponent|AddControlPointPosition _interptomovement (Transformation|GetWorldLocation (Variables|Default|GetPollen)) false)
  (Class|InterptoMovementComponent|AddControlPointPosition (Variables|Default|GetInterpToMovement) (Math|Vector|MakeVector (+ (.x _returnvalue_5) (Math|Random|RandomFloatinRange -75.0 75.0)) (+ (.y _returnvalue_5) (Math|Random|RandomFloatinRange -75.0 75.0)) (+ (.z _returnvalue_5) (Math|Random|RandomFloatinRange -75.0 75.0))) false)
  (if (Variables|Default|GetInstantTimerElapsed)
    (Class|InterptoMovementComponent|FinaliseControlPoints (Variables|Default|GetInterpToMovement))
    (else
      (if (>= _returnvalue_7 0.3)
        (Variables|/Script/Engine.InterpToMovementComponent|SetDuration _interptomovement_2 0.1)
        (else
          (Variables|/Script/Engine.InterpToMovementComponent|SetDuration _interptomovement_2 _returnvalue_7)))
      (Class|InterptoMovementComponent|FinaliseControlPoints _interptomovement_2))))

(fn SetMaterialColors
  (params (LightShade :type Linear%20Color%20Structure) (DarkDeepShade :type Linear%20Color%20Structure) (Material :type Material%20Instance%20Dynamic%20Object%20Reference))
  (Rendering|Material|SetVectorParameterValue Material "ColorFade_1" LightShade :!class /Script/Engine.MaterialInstanceDynamic)
  (Rendering|Material|SetVectorParameterValue Material "ColorFade_2" DarkDeepShade :!class /Script/Engine.MaterialInstanceDynamic))

(fn GetMaterialColors
  (bind _orb_material (Variables|Default|GetOrb_Material))
  (bind _returnvalue (Rendering|Material|GetVectorParameterValue _orb_material "ColorFade_1" :!class /Script/Engine.MaterialInstanceDynamic))
  (bind _returnvalue_2 (Rendering|Material|GetVectorParameterValue _orb_material "ColorFade_2" :!class /Script/Engine.MaterialInstanceDynamic))
  (return _returnvalue _returnvalue_2))

(fn SetupTrailColor
  (bind _n_trail (Variables|Default|GetN_Trail))
  (bind (_colormin _colormax) (CallFunction|GetMaterialColors))
  (Niagara|SetNiagaraVariable(LinearColor) _n_trail "ColorMin" _colormin)
  (Niagara|SetNiagaraVariable(LinearColor) _n_trail "ColorMax" _colormax))

(fn ResourceIncrease
  (bind _outactors (Actor|GetAllActorsOfClass "/Game/pollen_collect/ResourceManager/BP_ResourceManager.BP_ResourceManager_C"))
  (Default|AddNectar (Utilities|Array|Get(acopy) _outactors))
  (Default|AddPollen (Utilities|Array|Get(acopy) _outactors) (Variables|/Game/pollen_collect/Pollen/BP_PollenAura.BP_PollenAura_C|GetpollenID (Variables|Default|GetParentAura))))

(fn NodesRandomRoam
  (bind _parentaura (Variables|Default|GetParentAura))
  (bind _interptomovement (Variables|Default|GetInterpToMovement))
  (bind _interptomovement_2 (Variables|Default|GetInterpToMovement))
  (bind _sphere (Variables|/Game/pollen_collect/Pollen/BP_PollenAura.BP_PollenAura_C|GetSphere _parentaura))
  (bind (_origin _boxextent) (Collision|GetComponentBounds _sphere))
  (Class|InterptoMovementComponent|ResetControlPoints _interptomovement)
  (Class|InterptoMovementComponent|AddControlPointPosition _interptomovement (Transformation|GetWorldLocation (Variables|Default|GetPollen)) false)
  (for _index (range 0 4)
    (Class|InterptoMovementComponent|AddControlPointPosition (Variables|Default|GetInterpToMovement) (Math|Random|RandomPointinBoundingBox _origin _boxextent) false))
  (Class|InterptoMovementComponent|FinaliseControlPoints _interptomovement_2)
  (Variables|/Script/Engine.InterpToMovementComponent|SetDuration _interptomovement_2 (Math|Random|RandomFloatinRange 9e+01 1.5e+02))
  (Class|InterptoMovementComponent|RestartMovement _interptomovement_2 1.0))

(fn SetParentAura
  (params (ParentAura :type BP%20Pollen%20Aura%20Object%20Reference))
  (Variables|Default|SetParentAura ParentAura))

(fn AddNectar
  (return false))

(fn AddPollen
  (params (ID :type Float%20%28double-precision%29))
  (return))

(fn PollenPickup
  (params (P_Orb :type BP%20Master%20Trail%20Orb%20Object%20Reference))
  (return false))