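; Pollen aura around a plant that spawns roaming pollen and nectar orbs and handles pollination by the player.
; MainSetup spawns the initial orbs and starts looping timers that add more, each registered in OwnOrbs with a color-matched BP_PollenCollect.
; Orb spawns and pickups resize the sphere and update the Niagara radius and spawn rate.
; Player overlap alerts owned orbs and checks PollenID with the character to pollinate ParentPlant.
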(event OnComponentBeginOverlap(Sphere)
  (params (OverlappedComponent :type Primitive%20Component%20Object%20Reference) (OtherActor :type Actor%20Object%20Reference) (OtherComp :type Primitive%20Component%20Object%20Reference) (OtherBodyIndex :type Integer) (bFromSweep :type Boolean) (SweepResult :type Hit%20Result%20Structure%20%28by%20ref%29))
  (if (== OtherActor (Game|GetPlayerCharacter 0))
    (CallFunction|CheckPollinate)
    (CallFunction|PlayerTriggerOverlap)))

(event EventBeginPlay
  (Variables|Default|SetpollenID (Math|Random|RandomFloat)))

(event Collision|EventActorBeginOverlap
  (params (OtherActor :type Actor%20Object%20Reference)))

(event EventTick
  (params (DeltaSeconds :type Float%20%28single-precision%29)))

(fn ConstructionScript)

(fn PlayerTriggerOverlap
  (for _array_element (Variables|Default|GetOwnOrbs)
    (if (Utilities|IsValid _array_element)
      (Default|BeeinRadius _array_element))))

(fn MainSetup
  (params (PollenCount_OnSpawn :type Integer) (NectarCount_OnSpawn :type Integer) (Cooldown_PollenCount :type Integer) (Cooldown_NectarCount :type Integer) (PollenCooldown :type Float%20%28double-precision%29) (NectarCooldown :type Float%20%28double-precision%29) (DefaultScale :type Vector))
  (Utilities|FlowControl|Sequence
    (:then_0
      (Variables|Default|SetPollenCount Cooldown_PollenCount)
      (Variables|Default|SetNectar%20Count Cooldown_NectarCount)
      (Variables|Default|SetPollen_Cooldown PollenCooldown)
      (Variables|Default|SetNectar%20Cooldown NectarCooldown)
      (Variables|Scale|SetDefaultScale DefaultScale))
    (:then_1
      (for _index (range 0 (- PollenCount_OnSpawn 1))
        (Spawn|SpawnNewPollen))
      (for _index_2 (range 0 (- NectarCount_OnSpawn 1))
        (Spawn|SpawnNewNectar)))
    (:then_2
      ;[0.15 0.15 0.15 0.5] Sets Up Timer to handle Cooldown
      (Utilities|Time|SetTimerbyFunctionName 0 "Timer_PollenCooldownSpawn" (Variables|Default|GetPollen_Cooldown) true)
      (Utilities|Time|SetTimerbyFunctionName 0 "Timer_NectarCooldownSpawn" (Variables|Default|GetNectar%20Cooldown) true)
      (Update|UpdateScale))))

(fn SpawnNewPollen
  (bind _sphere (Variables|Default|GetSphere))
  (bind (_origin _boxextent) (Collision|GetComponentBounds _sphere))
  (Utilities|FlowControl|Sequence
    (:then_0
      (Variables|Scale|SetScaleIncrease (+ (Variables|Scale|GetScaleIncrease) 0.6))
      ;[0.15 0.15 0.15 0.5] Creates New Pollen Orb | Sets self as it's parent so that it may be easily called later (Get Actor would be inefficient due to there being multiple PollenAura Instances | Adds Pollen Orb to OwnPollen so that they can be triggered globaly
      (Update|UpdateScale)
      (bind _returnvalue (Game|SpawnActorfromClass "/Game/pollen_collect/Pollen/BP_Orb_Pollen.BP_Orb_Pollen_C" (Math|Transform|MakeTransform (Math|Random|RandomPointinBoundingBox _origin _boxextent) "0, 0, 0" "1.000000,1.000000,1.000000") "Undefined" "MultiplyWithRoot" 0 self 0))
      (CallFunction|ArrayAddOrb _returnvalue)
      (if (Utilities|IsValid _returnvalue)
        (Default|NodesRandomRoam _returnvalue)))
    (:then_1
      (Update|UpdateNiagaraValues))))

(fn TimerPollenCooldownSpawn
  (for _index (range 0 (- (Variables|Default|GetPollenCount) 1))
    (Spawn|SpawnNewPollen)))

(fn UpdateNiagaraValues
  (if (< (Variables|Niagara|GetAura_SpawnRate) 0.0)
    (Variables|Niagara|SetAura_SpawnRate 0.0))
  (if (> (Variables|Niagara|GetAura_SpawnRate) 49.0)
    (Variables|Niagara|SetAura_SpawnRate 49.0)
    (else
      (Variables|Niagara|SetAura_SpawnRate (* (+ (Utilities|Array|LastIndex (Variables|Default|GetOwnOrbs)) 1) 7.0))))
  (Niagara|SetNiagaraVariable(Float) (Variables|Default|GetN_PollenRadius) "UserSpawnRate" (Variables|Niagara|GetAura_SpawnRate))
  (Niagara|SetNiagaraVariable(Float) (Variables|Default|GetN_PollenRadius) "UserSphereRadius" (/ (* (+ (.x (Variables|Scale|GetDefaultScale)) (Variables|Scale|GetScaleIncrease)) 1e+02) 2.0)))

(fn UpdateScale
  (bind _scaleincrease (Variables|Scale|GetScaleIncrease))
  (Transformation|SetWorldScale3D (Variables|Default|GetSphere) (+ (Variables|Scale|GetDefaultScale) (Math|Vector|MakeVector _scaleincrease _scaleincrease _scaleincrease))))

(fn ArrayAddOrb
  (params (OrbToAdd :type BP%20Master%20Trail%20Orb%20Object%20Reference))
  (if (Utilities|IsValid OrbToAdd)
    (Utilities|Array|Add (Variables|Default|GetOwnOrbs) OrbToAdd)
    (bind _returnvalue (Game|SpawnActorfromClass "/Game/pollen_collect/Pollen/BP_PollenCollect.BP_PollenCollect_C" (Transformation|GetActorTransform OrbToAdd) "Undefined" "MultiplyWithRoot" 0 0))
    (bind (_colormin _colormax) (Default|GetMaterialColors OrbToAdd))
    (Default|SetupColor _returnvalue _colormin _colormax)))

(fn SpawnNewNectar
  (bind _sphere (Variables|Default|GetSphere))
  (bind (_origin _boxextent) (Collision|GetComponentBounds _sphere))
  (Utilities|FlowControl|Sequence
    (:then_0
      (Variables|Scale|SetScaleIncrease (+ (Variables|Scale|GetScaleIncrease) 0.6))
      ;[0.15 0.15 0.15 0.5] Creates New Pollen Orb | Sets self as it's parent so that it may be easily called later (Get Actor would be inefficient due to there being multiple PollenAura Instances | Adds Pollen Orb to OwnPollen so that they can be triggered globaly
      (Update|UpdateScale)
      (bind _returnvalue (Game|SpawnActorfromClass "/Game/pollen_collect/Pollen/BP_Orb_Nectar.BP_Orb_Nectar_C" (Math|Transform|MakeTransform (Math|Random|RandomPointinBoundingBox _origin _boxextent) "0, 0, 0" "1.000000,1.000000,1.000000") "Undefined" "MultiplyWithRoot" 0 self 0))
      (CallFunction|ArrayAddOrb _returnvalue)
      (if (Utilities|IsValid _returnvalue)
        (Default|NodesRandomRoam _returnvalue)))
    (:then_1
      (Update|UpdateNiagaraValues))))

(fn TimerNectarCooldownSpawn
  (for _index (range 0 (- (Variables|Default|GetNectar%20Count) 1))
    (Spawn|SpawnNewNectar)))

(fn CheckPollinate
  (bind _success (Class|IFPollination|Pollinate(Message) (Game|GetPlayerCharacter 0) (Variables|Default|GetpollenID)))
  (if _success
    (Default|Pollinated (Variables|Default|GetparentPlant))))

(fn AddNectar
  (return false))

(fn AddPollen
  (params (ID :type Float%20%28double-precision%29))
  (return))

(fn PollenPickup
  (params (P_Orb :type BP%20Master%20Trail%20Orb%20Object%20Reference))
  ;[0.15 0.15 0.15 0.5] Removed Pollen from array and reduces the scale increase
  (Utilities|Array|RemoveItem (Variables|Default|GetOwnOrbs) P_Orb)
  (Variables|Scale|SetScaleIncrease (- (Variables|Scale|GetScaleIncrease) 0.6))
  (Update|UpdateScale)
  (Update|UpdateNiagaraValues)
  (return false))