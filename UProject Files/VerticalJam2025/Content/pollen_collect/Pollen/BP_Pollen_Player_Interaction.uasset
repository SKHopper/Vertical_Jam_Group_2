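; BP_Pollen_Player_Interaction is an early scaffold for player interaction with pollen and nectar resources.
; On BeginPlay it spawns a BP_ResourceManager, stores it, and assigns it to the player's BP_TopDownCharacter.
; AddNectar, AddPollen and PollenPickup are stubs that return false, and TestSelf is empty.
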(event EventBeginPlay
  (CallFunction|ConstructResourceManager))

(event EventTick
  (params (DeltaSeconds :type Float%20%28single-precision%29)))

(fn TestSelf
  (return 0))

(fn ConstructResourceManager
  (bind _returnvalue (Game|SpawnActorfromClass "/Game/pollen_collect/ResourceManager/BP_ResourceManager.BP_ResourceManager_C" (Math|Transform|MakeTransform "0, 0, 0" "0, 0, 0" "1.000000,1.000000,1.000000") "Undefined" "MultiplyWithRoot" 0 0))
  (bind _output_get (Variables|Default|SetResourceManager _returnvalue))
  (bind _asbp_top_down_character (Utilities|Casting|CastToBP_TopDownCharacter (Game|GetPlayerCharacter 0)))
  (Variables|/Game/TopDown/Blueprints/BP_TopDownCharacter.BP_TopDownCharacter_C|SetresourceManager _asbp_top_down_character _output_get))

(fn AddNectar
  (return false))

(fn AddPollen
  (return false))

(fn PollenPickup
  (params (P_Orb :type BP%20Master%20Trail%20Orb%20Object%20Reference))
  (return false))