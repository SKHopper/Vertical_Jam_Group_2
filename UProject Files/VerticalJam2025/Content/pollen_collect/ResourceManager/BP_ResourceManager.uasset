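; BP_ResourceManager tracks collected nectar and pollen totals and shows them on a WID_Resource HUD widget, created from the construction script.
; Add functions increment the totals and refresh the widget, with pollen also recording unique source IDs.
; DepositeNectar returns and zeroes nectar without refreshing the widget.
; PollenPickup is a stub, and Pollinate checks stored IDs but always returns false due to a constant false in its condition.
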(fn ConstructionScript
  (CallFunction|ConstructWidget))

(fn ConstructWidget
  (bind _returnvalue (UserInterface|CreateWidget "/Game/pollen_collect/ResourceManager/WID_Resource.WID_Resource_C"))
  (bind _output_get (Variables|Default|SetResWidget _returnvalue))
  (UserInterface|Viewport|AddtoViewport _output_get 0)
  (Default|SetNectarCount _output_get (Variables|Default|GetNectarTotal))
  (Default|SetPollenCount _output_get (Variables|Default|GetPollenTotal)))

(fn AddNectar
  (bind _result (Math|Float|IncrementFloat (Variables|Default|GetNectarTotal))
    (:%20%20
      (Default|SetNectarCount (Variables|Default|GetResWidget) _result)
      (return false))))

(fn AddPollen
  (params (ID :type Float%20%28double-precision%29))
  (Utilities|Array|AddUnique (Variables|Default|GetpollenIDs) ID)
  (bind _result (Math|Float|IncrementFloat (Variables|Default|GetPollenTotal))
    (:%20%20
      (Default|SetPollenCount (Variables|Default|GetResWidget) _result)
      (return))))

(fn DepositeNectar
  (bind _output_get (LocalVariables|Setdeposite (Variables|Default|GetNectarTotal)))
  (Variables|Default|SetNectarTotal 0.0)
  (return _output_get))

(fn PollenPickup
  (params (P_Orb :type BP%20Master%20Trail%20Orb%20Object%20Reference))
  (return false))

(fn Pollinate
  (params (ID :type Float%20%28double-precision%29))
  (bind _pollenids (Variables|Default|GetpollenIDs))
  (bind _returnvalue (Utilities|Array|Length _pollenids))
  (if (Math|Boolean|ANDBoolean (Math|Conversions|ToBoolean(Integer) _returnvalue) (or (> _returnvalue 1) (not (Utilities|Array|ContainsItem _pollenids ID))) false)
    (return true)
    (else
      (return false))))