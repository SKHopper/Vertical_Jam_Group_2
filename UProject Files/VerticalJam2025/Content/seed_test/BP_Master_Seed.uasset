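; BP_Master_Seed is a seed actor that grows into a flower chosen by its species data.
; On hit, the Seed component stops simulating physics and starts a timer, with no bound event shown.
; SeedGrow looks up the SpeciesData row, spawns its FlowerType at the actor's transform and destroys the seed.
; SeedPlant spawns a BP_Seed_Child at the Seed component's transform and passes it SpeciesData through MainSetup.
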(event OnComponentHit(Seed)
  (params (HitComponent :type Primitive%20Component%20Object%20Reference) (OtherActor :type Actor%20Object%20Reference) (OtherComp :type Primitive%20Component%20Object%20Reference) (NormalImpulse :type Vector :default "0, 0, 0") (Hit :type Hit%20Result%20Structure%20%28by%20ref%29))
  (Physics|SetSimulatePhysics (Variables|Default|GetSeed) false)
  (Utilities|Time|SetTimerbyEvent 0 0.0))

(fn ConstructionScript)

(fn SeedGrow
  (bind _species_data (Variables|Default|GetSpecies_Data))
  (bind _returnvalue (Utilities|GetDataTableRow (.datatable _species_data) (.rowname _species_data))
    (:then
      (Game|SpawnActorfromClass (.FlowerType (Utilities|Struct|BreakSTRUCT_TESTFLOWER _returnvalue)) (Transformation|GetActorTransform) "Undefined" "MultiplyWithRoot" 0 0)
      (Actor|DestroyActor))))

(fn SeedPlant
  (bind _returnvalue (Game|SpawnActorfromClass :Class "/Game/seed_test/BP_Seed_Child.BP_Seed_Child_C" :SpawnTransform (Transformation|GetWorldTransform (Variables|Default|GetSeed)) :CollisionHandlingOverride "Undefined" :TransformScaleMethod "MultiplyWithRoot" :Instigator 0))
  (Default|MainSetup _returnvalue (Variables|Default|GetSpecies_Data)))